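; BP_MainCharacter is the main character Blueprint, with a two-key shortcut that opens the end screen.
; Escape and D key events set held-state flags on press and clear them on release.
; Tick polls both flags and, while both are held, creates a new WBP_EndScreen every frame, adds it to the viewport and shows the mouse cursor.
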(event `self.ReceiveBeginPlay`)

(event `self.ReceiveTick`
  (params (DeltaSeconds :type "Float (single-precision)"))
  (if (and (`self.IsD`) (`self.IsEsc`))
    (bind _returnvalue (`|CreateWidget` "/Game/UI/WBP_EndScreen.WBP_EndScreen_C"))
    (`UserWidget.AddToViewport` _returnvalue 0)
    (set `PlayerController.bShowMouseCursor` true (`GameplayStatics.GetPlayerController` 0))))

(event `Key|Escape`
  (params (Key :type "Key Structure"))
  (:`Pressed`
    (set `self.IsEsc` true))
  (:`Released`
    (set `self.IsEsc` false)))

(event `Key|D`
  (params (Key :type "Key Structure"))
  (:`Pressed`
    (set `self.IsD` true))
  (:`Released`
    (set `self.IsD` false)))

(fn `UserConstructionScript`)